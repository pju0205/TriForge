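; BP_TFPlayerCharacter2 is a player character Blueprint that handles sniper scope feedback and foley audio.
; ShowSniperScope lazily creates the scope widget, then plays its zoom animation forward or reversed with matching zoom sounds.
; Jump and land events play gameplay-tagged sounds from a default foley audio bank at the mesh location, scaling volume by horizontal speed or landing velocity.
; Footstep sounds are allowed only while moving on the ground.
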(event EventOnJumped
  (Audio|PlayAudioEvent "(TagName=\"Foley.Event.Jump\")" (Math|Float|MapRangeClamped (Math|Vector|VectorLengthXY (Variables|/Script/Engine.MovementComponent|GetVelocity (Variables|Character|GetCharacterMovement))) 0.0 5e+02 0.5 1.0) 1.0))

(event EventOnLanded
  (params (Hit :type Hit%20Result%20Structure%20%28by%20ref%29))
  (Audio|PlayAudioEvent "(TagName=\"Foley.Event.Land\")" (Math|Float|MapRangeClamped (.z (Variables|Default|GetLandVelocity)) -5e+02 -9e+02 0.5 1.5) 1.0))

(event EventShowSniperScope
  (params (bShowScope :type Boolean))
  ;[1 1 1] Add SniperScope to ViewPort  bShowScope true = PlayAnimation Forward, false = PlayAnimation Reverse
  (Utilities|IsValid (Variables|Default|GetSniperScopeWidget)
    (:Is%20Valid
      _)
    (:Is%20Not%20Valid
      (bind _returnvalue (UserInterface|CreateWidget "/Game/Game/UI/Blueprint/HUD/WBP_SniperScope.WBP_SniperScope_C"))
      (bind _output_get (Variables|Default|SetSniperScopeWidget _returnvalue))
      (UserInterface|Viewport|AddtoViewport _output_get 0)))
  (if bShowScope
    (Utilities|IsValid (Variables|Default|GetSniperScopeWidget)
      (:Is%20Valid
        (UserInterface|Animation|PlayAnimation (Variables|Default|GetSniperScopeWidget) (Variables|/Game/Game/UI/Blueprint/HUD/WBP_SniperScope.WBP_SniperScope_C|GetScopeZoomIn (Variables|Default|GetSniperScopeWidget)) 0.0 1 "Forward" 1.0 false)
        (Audio|PlaySound2D "/Game/Assets/WeaponAssets/MilitaryWeapSilver/Sound/SniperRifle/Cues/SniperRifle_ZoomIn_Cue.SniperRifle_ZoomIn_Cue" 1.0 1.0 0.0 0 0)))
    (else
      (Utilities|IsValid (Variables|Default|GetSniperScopeWidget)
        (:Is%20Valid
          (UserInterface|Animation|PlayAnimation (Variables|Default|GetSniperScopeWidget) (Variables|/Game/Game/UI/Blueprint/HUD/WBP_SniperScope.WBP_SniperScope_C|GetScopeZoomIn (Variables|Default|GetSniperScopeWidget)) 0.0 1 "Reverse" 1.0 false)
          (Audio|PlaySound2D "/Game/Assets/WeaponAssets/MilitaryWeapSilver/Sound/SniperRifle/Cues/SniperRifle_ZoomOut_Cue.SniperRifle_ZoomOut_Cue" 1.0 1.0 0.0 0 0))))))

(fn ConstructionScript)

(fn PlayAudioEvent
  (params (Value :type Gameplay%20Tag%20Structure) (VolumeMultiplier :type Float%20%28double-precision%29) (PitchMultiplier :type Float%20%28double-precision%29))
  (bind _foleyaudiobank (CallFunction|GetFoleyAudioBank))
  (Audio|PlaySoundatLocation (.Sound (Default|GetSoundfromFoleyEvent _foleyaudiobank Value)) (Transformation|GetWorldLocation (Variables|Character|GetMesh)) "0, 0, 0" VolumeMultiplier PitchMultiplier 0.0 0 0 0 0))

(fn CanPlayFootstepSounds
  (return (AI|Components|NavMovement|IsMovingonGround (Variables|Character|GetCharacterMovement))))

(fn GetFoleyAudioBank
  (return "/Game/Characters/Audio/Foley/DefaultFoleyEventAudioBank.DefaultFoleyEventAudioBank"))